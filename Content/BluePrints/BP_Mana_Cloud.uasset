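; BP_Mana_Cloud is a mana pickup that adds a random amount of mana to the ThirdPersonCharacter's cloud mana pool on overlap.
; On BeginPlay it rolls a small whole-number value, shows it as text and derives the cloud particle's X scale from it, zeroing Y and Z.
; Overlap adds the value, deactivates the particle, prints the total and destroys the actor after a delay, with collision left active meanwhile.
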(event OnComponentBeginOverlap(ManaCloudCollision)
  (params (OverlappedComponent :type Primitive%20Component%20Object%20Reference) (OtherActor :type Actor%20Object%20Reference) (OtherComp :type Primitive%20Component%20Object%20Reference) (OtherBodyIndex :type Integer) (bFromSweep :type Boolean) (SweepResult :type Hit%20Result%20Structure%20%28by%20ref%29))
  ;[1 1 1] On intersect, adds instance's Mana value to character cloud mana pool, then destroys actor
  (bind _asthird_person_character (Utilities|Casting|CastToThirdPersonCharacter OtherActor))
  (bind _output_get (Variables|/Game/ThirdPersonBP/Blueprints/ThirdPersonCharacter.ThirdPersonCharacter_C|SetMana_Character_Cloud_Value _asthird_person_character (Math|Conversions|ToFloat(Integer) (+ (Math|Float|Truncate (Variables|/Game/ThirdPersonBP/Blueprints/ThirdPersonCharacter.ThirdPersonCharacter_C|GetMana_Character_Cloud_Value _asthird_person_character)) (stale EventBeginPlay _output_get)))))
  (Components|Activation|Deactivate (Variables|Default|GetP_ManaCloud))
  (Development|PrintString (Utilities|String|ToString(Float) _output_get))
  (Utilities|FlowControl|Delay 5.0)
  (Actor|DestroyActor))

(event EventBeginPlay
  ;[1 1 1] Randomly Sets Instance's Mana Value and Renders Value Above Actor
  (bind _output_get (Variables|Default|SetMana_Cloud_Value (Math|Float|Truncate (Math|Random|RandomFloatinRange 1.0 5.0))))
  (Rendering|Components|TextRender|SetText (Variables|Default|GetCloud_Mana_Value_Text) (Utilities|Text|ToText(Integer) _output_get))
  ;[1 1 1] Using Mana Cloud Value, sets X-axix scale of particle
  (Transformation|SetWorldScale3D (Variables|Default|GetP_ManaCloud) (Math|Vector|MakeVector (Math|Conversions|ToFloat(Integer) (+ (/ _output_get 3) 1)) 0.0 0.0)))

(fn ConstructionScript)